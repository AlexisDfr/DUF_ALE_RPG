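; BP_PNJ is an interactable NPC actor that toggles a dialogue-style view when the player interacts with it.
; The Interact event alternates through a FlipFlop: first it shows a text render, blends the camera to the NPC and disables movement through the top-down controller's ShouldMove flag.
; The next interaction hides the text, blends the view back to the controlled pawn and re-enables movement.
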(event EventBeginPlay
  (|CallParentFunction) ; This node is disabled and will not be called.\nDrag off pins to build functionality.
)

(event Collision|EventActorBeginOverlap
  (params (OtherActor :type Actor%20Object%20Reference)))

(event EventTick
  (params (DeltaSeconds :type Float%20%28single-precision%29))
  (|CallParentFunction DeltaSeconds) ; This node is disabled and will not be called.\nDrag off pins to build functionality.
)

(event EventInteract
  (bind _playercontroller (CallFunction|GetTopDownController))
  (bind _playercontroller_2 (CallFunction|GetTopDownController))
  (Utilities|FlowControl|FlipFlop
    (:A
      (Rendering|SetVisibility (Variables|Default|GetTextRender1) true false)
      (Game|Player|SetViewTargetwithBlend _playercontroller_2 self 1.0 "VTBlend_Linear" 1.0 false)
      (Variables|/Game/Blueprint/TopDown/BP_TopDownController.BP_TopDownController_C|SetShouldMove _playercontroller_2 false))
    (:B
      (Rendering|SetVisibility (Variables|Default|GetTextRender1) false false)
      (Game|Player|SetViewTargetwithBlend _playercontroller (Pawn|GetControlledPawn _playercontroller) 1.0 "VTBlend_Linear" 0.0 false)
      (Variables|/Game/Blueprint/TopDown/BP_TopDownController.BP_TopDownController_C|SetShouldMove _playercontroller true))))

(fn ConstructionScript
  (|CallParentFunction))